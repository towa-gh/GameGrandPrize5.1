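; BP_FallingFloar is a floor that drops shortly after the player character steps into its trigger box, then returns to its original place.
; A timer after the overlap turns on physics simulation on the static mesh, and a second timer resets it.
; The reset disables physics, reattaches the mesh to the root (simulation detaches it), and restores the relative location and rotation cached at BeginPlay.
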(event `self.ReceiveBeginPlay`
  (bind _staticmesh (`self.StaticMesh`))
  (set `self.New Location` (`SceneComponent.RelativeLocation` _staticmesh))
  (set `self.New Rotation` (`SceneComponent.RelativeRotation` _staticmesh)))

(event `self.Box.OnComponentBeginOverlap`
  (params (OverlappedComponent :type "PrimitiveComponent Object Reference") (OtherActor :type "Actor Object Reference") (OtherComp :type "PrimitiveComponent Object Reference") (OtherBodyIndex :type Integer) (bFromSweep :type Boolean) (SweepResult :type "HitResult Structure (by ref)"))
  (if (== OtherActor (`GameplayStatics.GetPlayerCharacter` 0))
    (`KismetSystemLibrary.K2_SetTimerDelegate` (delegate `CallFall`) 1.0)))

(event `CallFall`
  (`PrimitiveComponent.SetSimulatePhysics` (`self.StaticMesh`) true)
  (`KismetSystemLibrary.K2_SetTimerDelegate` (delegate `Reset Floar`) 1.0))

(event `Reset Floar`
  (`PrimitiveComponent.SetSimulatePhysics` (`self.StaticMesh`) false)
  (`SceneComponent.K2_AttachToComponent` (`self.StaticMesh`) (`self.DefaultSceneRoot`) "None" "KeepRelative" "KeepRelative" "KeepRelative" true)
  (`SceneComponent.K2_SetRelativeLocationAndRotation` (`self.StaticMesh`) (`self.New Location`) (`self.New Rotation`) false false))

(fn `UserConstructionScript`)